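; Player HUD Blueprint that creates the sidebar display and shows it only in the Game level.
; On BeginPlay it creates a SidebarDisplay widget, stores a reference, adds it to the viewport and sets game-only input for the first player controller.
; It then compares the current level name to Game to make the sidebar visible or hidden.
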(event `self.ReceiveBeginPlay`
  (bind _returnvalue (`|CreateWidget` "/Game/Blueprints/SidebarDisplay.SidebarDisplay_C"))
  (bind _output_get (set `self.SideBarReference` _returnvalue))
  (`UserWidget.AddToViewport` _output_get 0)
  (`WidgetBlueprintLibrary.SetInputMode_GameOnly` (`GameplayStatics.GetPlayerController` 0))
  (bind _returnvalue_2 (`GameplayStatics.GetCurrentLevelName` true))
  (bind _output_get_2 (set `self.CurrentLevel` _returnvalue_2))
  (if (== _output_get_2 (`self.Game`))
    (`Widget.SetVisibility` (`self.SideBarReference`) "Visible")
    (else
      (`Widget.SetVisibility` (`self.SideBarReference`) "Hidden"))))

(fn `UserConstructionScript`)