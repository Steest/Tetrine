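; Tetris-style player Blueprint that reacts to drop and save inputs with sidebar display animations.
; BeginPlay checks for a Player_HUD, but sets PlayerHUDRef to None before reading GameBoyHUD from it.
; InstantDrop, when IsInstantDropped is set, plays the landing animation, flags it started and records the current tetromino's shape.
; SaveTetro, unless BhasSavedTetromino is set, plays a ping-pong swap animation when a piece is held, otherwise the store animation.
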(event `self.ReceiveBeginPlay`
  (cast `/Game/Blueprints/Player_HUD` (`PlayerController.GetHUD` (`GameplayStatics.GetPlayerController` 0)))
  (bind _output_get (set `self.PlayerHUDRef` null))
  (set `self.GameBoyRef` (`/Game/Blueprints/MainHUD.GameBoyHUD` _output_get)))

(event `InputAction|InstantDrop` :overrideparent false
  (params (Key :type "Key Structure" :default "AnyKey"))
  (:`Pressed`
    (if (`self.bIsInstantDropped`)
      (`UserWidget.PlayAnimation` (`self.SidebarDisplay`) (`/Game/Blueprints/SidebarDisplay.LandedTetromino_anim` (`self.SidebarDisplay`)) 0.0 1 "Forward")
      (set `self.bHasStartedLandAnim` true)
      (set `self.CurrentTetrominoName` (`Tetromino.Shape` (`self.CurrentTetromino`))))))

(event `InputAction|SaveTetro` :overrideparent false
  (params (Key :type "Key Structure" :default "AnyKey"))
  (:`Pressed`
    (if (`self.bhasSavedTetromino`)
      _
      (elif (`KismetStringLibrary.NotEqual_StrStr` (`self.SavedTetromino`) "none")
        (`UserWidget.PlayAnimation` (`self.SidebarDisplay`) (`/Game/Blueprints/SidebarDisplay.Swap_anim` (`self.SidebarDisplay`)) 0.0 1 "PingPong")
        (else
          (`UserWidget.PlayAnimation` (`self.SidebarDisplay`) (`/Game/Blueprints/SidebarDisplay.Store_anim` (`self.SidebarDisplay`)) 0.0 1 "Forward"))))))

(fn `UserConstructionScript`)