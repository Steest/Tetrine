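; BP_Tetrine is a Blueprint that records a high score for what appears to be a Tetris-style game.
; On BeginPlay it casts the first player pawn to Possessor and stores the reference.
; Each Tick, once that pawn flags game over, it raises HighScore to the pawn's Lines count if that count is higher.
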(event `self.ReceiveBeginPlay`
  (bind _aspossessor (cast `Possessor` (`GameplayStatics.GetPlayerPawn` 0)))
  (set `self.MyPossessor` _aspossessor))

(event `self.ReceiveTick`
  (params (DeltaSeconds :type "Float (single-precision)"))
  (if (`Possessor.bIsGameOver` (`self.MyPossessor`))
    (if (> (`Possessor.Lines` (`self.MyPossessor`)) (`self.HighScore`))
      (set `self.HighScore` (`Possessor.Lines` (`self.MyPossessor`))))))

(fn `UserConstructionScript`)