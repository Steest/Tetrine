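; Extended possessor Blueprint for a Tetris-style game, linking tetromino play to the HUD sidebar display.
; On BeginPlay it casts the first player controller's HUD to Player_HUD and caches its sidebar widget.
; Logic for swap, store and instant-drop landing animations on that sidebar exists but is unwired, so it never runs.
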(event `self.ReceiveBeginPlay`
  (bind _asplayer_hud (cast `/Game/Blueprints/Player_HUD` (`PlayerController.GetHUD` (`GameplayStatics.GetPlayerController` 0))))
  (bind _output_get (set `self.PlayerHUDRef` _asplayer_hud))
  (set `self.SidebarDisplay` (`/Game/Blueprints/Player_HUD.SideBarReference` _output_get)))

(event `InputAction|InstantDrop` :overrideparent false
  (params (Key :type "Key Structure" :default "AnyKey")))

(event `InputAction|SaveTetro` :overrideparent false
  (params (Key :type "Key Structure" :default "AnyKey")))

(fn `UserConstructionScript`)